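; Game instance that holds a copy of each player's state data, with events to save and load it.
; SaveGameState copies StateData from every PlayerState_Main in the game state's PlayerArray into PlayerStateDataArray.
; LoadGameState writes it back, matching players purely by array index.
; A failed player state cast loops back through a short Delay to retry, from inside the ForEach loop.
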(event `SaveGameState`
  (bind _asgame_state_main (cast `/Game/shimabukuro/System/Blueprints/GameState_Main` (`GameplayStatics.GetGameState`)))
  (for (_array_element _array_index) (`GameStateBase.PlayerArray` _asgame_state_main)
    (bind _asplayer_state_main (cast `/Game/shimabukuro/System/Blueprints/PlayerState_Main` _array_element :!label _label)
      (:`then`
        (`KismetArrayLibrary.Array_Set` (`self.playerStateDataArray`) _array_index (`/Game/shimabukuro/System/Blueprints/PlayerState_Main.StateData` _asplayer_state_main) true))
      (:`CastFailed`
        (`KismetSystemLibrary.Delay` 0.2)
        (goto _label)))))

(event `LoadGameState`
  (bind _asgame_state_main (cast `/Game/shimabukuro/System/Blueprints/GameState_Main` (`GameplayStatics.GetGameState`)))
  (for (_array_element _array_index) (`GameStateBase.PlayerArray` _asgame_state_main)
    (bind _asplayer_state_main (cast `/Game/shimabukuro/System/Blueprints/PlayerState_Main` _array_element :!label _label_2)
      (:`then`
        (set `/Game/shimabukuro/System/Blueprints/PlayerState_Main.StateData` (`|GetArrayItem` (`self.playerStateDataArray`) _array_index) _asplayer_state_main))
      (:`CastFailed`
        (`KismetSystemLibrary.Delay` 0.2)
        (goto _label_2)))))