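; BP_ColorTile is a stage tile that takes on the team color of the player whose projectile hits it.
; On box overlap, while the match time is not up, it casts to BP_Projectile and reads the TeamID from the instigator's PlayerState_Main to set CurrentColor.
; CurrentColor's RepNotify swaps the plane's material between white, blue and orange, keeping the visual tied to replicated state.
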(event `self.Box.OnComponentBeginOverlap`
  (params (OverlappedComponent :type "PrimitiveComponent Object Reference") (OtherActor :type "Actor Object Reference") (OtherComp :type "PrimitiveComponent Object Reference") (OtherBodyIndex :type Integer) (bFromSweep :type Boolean) (SweepResult :type "HitResult Structure (by ref)"))
  (bind _asgame_state_main (cast `/Game/shimabukuro/System/Blueprints/GameState_Main` (`GameplayStatics.GetGameState`)))
  (if (not (`/Game/shimabukuro/System/Blueprints/GameState_Main.IsTimeUp` _asgame_state_main))
    (bind _asbp_projectile (cast `/Game/shimabukuro/Player/Blueprints/BP_Projectile` OtherActor))
    (bind _asplayer_state_main (cast `/Game/shimabukuro/System/Blueprints/PlayerState_Main` (`Pawn.PlayerState` (`self.GetInstigator` _asbp_projectile))))
    (bind (_statedata_ishost _statedata_isready _statedata_playername _statedata_teamid) (break `/Game/shimabukuro/System/Blueprints/Struct_PlayerStateData` (`/Game/shimabukuro/System/Blueprints/PlayerState_Main.StateData` _asplayer_state_main)))
    (switch `int` _statedata_teamid
      (:`1`
        (set `self.currentColor` 1))
      (:`2`
        (set `self.currentColor` 2)))))

(fn `OnRep_currentColor`
  (bind _plane (`self.Plane`))
  (switch `int` (`self.currentColor`)
    (:`0`
      (`PrimitiveComponent.SetMaterial` _plane 0 "/Game/shimabukuro/Stage/Materials/M_White.M_White"))
    (:`1`
      (`PrimitiveComponent.SetMaterial` _plane 0 "/Game/shimabukuro/Stage/Materials/M_Blue.M_Blue"))
    (:`2`
      (`PrimitiveComponent.SetMaterial` _plane 0 "/Game/shimabukuro/Stage/Materials/M_Orange.M_Orange"))))

(fn `UserConstructionScript`)