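; Game mode for the waiting room that handles host marking, the player cap and travel to the matching room.
; BeginPlay sets each PlayerState's host flag from its authority.
; PostLogin kicks the last PlayerArray entry when the count exceeds the GameInstance's MaxPlayers.
; OpenNextLevel locks MaxPlayers to the current count, saves game state through the GameInstance, then runs a one-shot servertravel to Level_MatchingRoom.
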(event `self.ReceiveBeginPlay`
  ;[1 1 1] ホストのPlayerStateに自分がホストであることを示す情報を保存
  (for _array_element (`GameStateBase.PlayerArray` (`GameplayStatics.GetGameState`))
    (bind _asplayer_state_main (cast `/Game/shimabukuro/System/Blueprints/PlayerState_Main` _array_element))
    (`/Game/shimabukuro/System/Blueprints/PlayerState_Main.SetHostState` _asplayer_state_main (`self.HasAuthority` _asplayer_state_main))))

(event `self.K2_PostLogin`
  (params (NewPlayer :type "PlayerController Object Reference"))
  (bind _returnvalue (`GameplayStatics.GetGameState`))
  ;[1 1 1] ログインがあったとき、プレイヤー数が上限に達していたときの自動キック処理
  (`|ExecutionSequence`
    (:`then_0`
      (bind _asgame_instance_main (cast `/Game/shimabukuro/System/Blueprints/GameInstance_Main` (`GameplayStatics.GetGameInstance`)))
      (bind _asgame_state_main (cast `/Game/shimabukuro/System/Blueprints/GameState_Main` _returnvalue))
      (bind _num (`/Game/shimabukuro/System/Blueprints/GameState_Main.GetCurrentPlayersNum` _asgame_state_main))
      (if (> _num (`/Game/shimabukuro/System/Blueprints/GameInstance_Main.MaxPlayers` _asgame_instance_main))
        (for _array_element (`GameStateBase.PlayerArray` _returnvalue)
          _)
        (bind _asplayer_controller_main (cast `/Game/shimabukuro/System/Blueprints/PlayerController_Main` (`PlayerState.GetPlayerController` _array_element)))
        (`/Game/shimabukuro/System/Blueprints/PlayerController_Main.Kick` _asplayer_controller_main)))))

(event `OpenNextLevel`
  ;[1 1 1] カスタムイベント - プレイヤー数上限の更新、GameStateを保存して次のレベルへ遷移する
  (`|ExecutionSequence`
    (:`then_0`
      (bind _asgame_instance_main (cast `/Game/shimabukuro/System/Blueprints/GameInstance_Main` (`GameplayStatics.GetGameInstance`)))
      (bind _asgame_state_main (cast `/Game/shimabukuro/System/Blueprints/GameState_Main` (`GameplayStatics.GetGameState`)))
      (bind _num (`/Game/shimabukuro/System/Blueprints/GameState_Main.GetCurrentPlayersNum` _asgame_state_main))
      (set `/Game/shimabukuro/System/Blueprints/GameInstance_Main.MaxPlayers` _num _asgame_instance_main))
    (:`then_1`
      (bind _asgame_instance_main_2 (cast `/Game/shimabukuro/System/Blueprints/GameInstance_Main` (`GameplayStatics.GetGameInstance`)))
      (`/Game/shimabukuro/System/Blueprints/GameInstance_Main.SaveGameState` _asgame_instance_main_2)
      (for _array_element (`GameStateBase.PlayerArray` (`GameplayStatics.GetGameState`))
        (if (`self.HasAuthority` _array_element)
          (`/Engine/EditorBlueprintResources/StandardMacros.DoOnce` false
            (:`Completed`
              (`KismetSystemLibrary.ExecuteConsoleCommand` (`KismetStringLibrary.Concat_StrStr` "servertravel " "/Game/shimabukuro/Menu/Maps/Level_MatchingRoom") (`PlayerState.GetPlayerController` _array_element)))))))))

(fn `UserConstructionScript`)