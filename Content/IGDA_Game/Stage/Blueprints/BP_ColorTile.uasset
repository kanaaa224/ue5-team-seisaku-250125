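; BP_ColorTile is a stage tile that turns transparent when a BP_Player overlaps its box.
; BeginPlay and the overlap set CurrentColor, whose RepNotify swaps the plane's material.
; The initial state picks a random black translucent material, weighted toward the base one, inside the notify rather than from a replicated value.
; A third state also maps to transparent but is never set here.
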(event `self.ReceiveBeginPlay`
  (set `self.currentColor` 0))

(event `self.Box.OnComponentBeginOverlap`
  (params (OverlappedComponent :type "PrimitiveComponent Object Reference") (OtherActor :type "Actor Object Reference") (OtherComp :type "PrimitiveComponent Object Reference") (OtherBodyIndex :type Integer) (bFromSweep :type Boolean) (SweepResult :type "HitResult Structure (by ref)"))
  (cast `/Game/IGDA_Game/Player/player/BP_Player` OtherActor)
  (set `self.currentColor` 1))

(fn `OnRep_currentColor`
  (bind _plane (`self.Plane`))
  (switch `int` (`self.currentColor`)
    (:`0`
      (switch `int` (`KismetMathLibrary.RandomInteger` 15)
        (:`Default`
          (`PrimitiveComponent.SetMaterial` _plane 0 "/Game/IGDA_Game/Stage/Materials/M_BlackTranslucent.M_BlackTranslucent"))
        (:`0`
          (`PrimitiveComponent.SetMaterial` _plane 0 "/Game/IGDA_Game/Stage/Materials/M_BlackTranslucent-1.M_BlackTranslucent-1"))
        (:`1`
          (`PrimitiveComponent.SetMaterial` _plane 0 "/Game/IGDA_Game/Stage/Materials/M_BlackTranslucent-2.M_BlackTranslucent-2"))
        (:`2`
          (`PrimitiveComponent.SetMaterial` _plane 0 "/Game/IGDA_Game/Stage/Materials/M_BlackTranslucent-3.M_BlackTranslucent-3"))
        (:`3`
          (`PrimitiveComponent.SetMaterial` _plane 0 "/Game/IGDA_Game/Stage/Materials/M_BlackTranslucent-4.M_BlackTranslucent-4"))
        (:`4`
          (`PrimitiveComponent.SetMaterial` _plane 0 "/Game/IGDA_Game/Stage/Materials/M_BlackTranslucent-5.M_BlackTranslucent-5"))))
    (:`1`
      (`PrimitiveComponent.SetMaterial` _plane 0 "/Game/IGDA_Game/Stage/Materials/M_Transparent.M_Transparent"))
    (:`2`
      (`PrimitiveComponent.SetMaterial` _plane 0 "/Game/IGDA_Game/Stage/Materials/M_Transparent.M_Transparent"))))

(fn `UserConstructionScript`)