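; Player controller that lets the player toggle between the soap character and a separate camera pawn.
; BeginPlay adds the Enhanced Input mapping context, caches the BP_Player pawn and spawns a BP_Camera high above the origin.
; The change-look input flip-flops possession, switching active cameras and hiding the soap mesh and disabling its collision while the camera is possessed.
; A separate ChangeCharacter function repeats the toggle without possessing.
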(event `self.ReceiveBeginPlay`
  (bind (_asbp_player _bsuccess) (cast `/Game/IGDA_Game/Player/player/BP_Player` (`GameplayStatics.GetPlayerPawn` 0) :!pure true))
  (`EnhancedInputSubsystemInterface.AddMappingContext` (subsystem `EnhancedInputLocalPlayerSubsystem`) "/Game/ThirdPerson/Input/IMC_Default.IMC_Default" 0 (struct))
  (if _bsuccess
    (set `self.soap` _asbp_player)
    (bind _returnvalue (`|SpawnActorFromClass` "/Game/IGDA_Game/Player/Camera/BP_Camera.BP_Camera_C" (`KismetMathLibrary.MakeTransform` (0.0 0.0 1000.0)) "Undefined" "MultiplyWithRoot" null null))
    (bind _output_get (set `self.camera_` _returnvalue))
    (`ActorComponent.SetActive` (`/Game/IGDA_Game/Player/Camera/BP_Camera.Camera` _output_get) false false)))

(event `EnhancedInput|/Game/ThirdPerson/Input/Actions/IA_ChageLook`
  (params (ActionValue :type Boolean) (ElapsedSeconds :type "Float (double-precision)") (TriggeredSeconds :type "Float (double-precision)") (InputAction :type "InputAction Object Reference" :default "/Game/ThirdPerson/Input/Actions/IA_ChageLook.IA_ChageLook"))
  (:`Started`
    (`/Engine/EditorBlueprintResources/StandardMacros.FlipFlop`
      (:`A`
        (`self.SetCharacterVisiblityAndCollision` false (`self.soap`))
        (`ActorComponent.SetActive` (`/Game/IGDA_Game/Player/player/BP_Player.Camera` (`self.soap`)) false false)
        (`ActorComponent.SetActive` (`/Game/IGDA_Game/Player/Camera/BP_Camera.Camera` (`self.camera_`)) true false)
        (`self.Possess` (`self.camera_`)))
      (:`B`
        (`self.SetCharacterVisiblityAndCollision` true (`self.soap`))
        (`ActorComponent.SetActive` (`/Game/IGDA_Game/Player/player/BP_Player.Camera` (`self.soap`)) true false)
        (`ActorComponent.SetActive` (`/Game/IGDA_Game/Player/Camera/BP_Camera.Camera` (`self.camera_`)) false false)
        (`self.Possess` (`self.soap`))))))

(fn `ChangeCharacter`
  (`/Engine/EditorBlueprintResources/StandardMacros.FlipFlop`
    (:`A`
      (`self.SetCharacterVisiblityAndCollision` false (`self.soap`))
      (`ActorComponent.SetActive` (`/Game/IGDA_Game/Player/player/BP_Player.Camera` (`self.soap`)) false false)
      (`ActorComponent.SetActive` (`/Game/IGDA_Game/Player/Camera/BP_Camera.Camera` (`self.camera_`)) true false))
    (:`B`
      (`self.SetCharacterVisiblityAndCollision` true (`self.soap`))
      (`ActorComponent.SetActive` (`/Game/IGDA_Game/Player/player/BP_Player.Camera` (`self.soap`)) true false)
      (`ActorComponent.SetActive` (`/Game/IGDA_Game/Player/Camera/BP_Camera.Camera` (`self.camera_`)) false false))))

(fn `SetCharacterVisiblityAndCollision`
  (params (` VisiblityAndCollision` :type Boolean) (Character :type "Character Object Reference"))
  (locals (TargetCharacter :type "/Game/IGDA_Game/Player/player/BP_Player Object Reference"))
  (bind _targetcharacter (`local.TargetCharacter`))
  (bind _targetcharacter_2 (`local.TargetCharacter`))
  (bind _soapmesh (`/Game/IGDA_Game/Player/player/BP_Player.SoapMesh` _targetcharacter))
  (bind _soapmesh_2 (`/Game/IGDA_Game/Player/player/BP_Player.SoapMesh` _targetcharacter_2))
  (bind _asbp_player (cast `/Game/IGDA_Game/Player/player/BP_Player` Character))
  (set `local.TargetCharacter` _asbp_player)
  (if ` VisiblityAndCollision`
    (`SceneComponent.SetVisibility` _soapmesh_2 true false)
    (`PrimitiveComponent.SetCollisionEnabled` (`Character.CapsuleComponent` _targetcharacter_2) "QueryAndPhysics")
    (`PrimitiveComponent.SetCollisionEnabled` _soapmesh_2 "QueryAndPhysics")
    (else
      (`SceneComponent.SetVisibility` _soapmesh false false)
      (`PrimitiveComponent.SetCollisionEnabled` (`Character.CapsuleComponent` _targetcharacter) "NoCollision")
      (`PrimitiveComponent.SetCollisionEnabled` _soapmesh "NoCollision"))))

(fn `UserConstructionScript`)