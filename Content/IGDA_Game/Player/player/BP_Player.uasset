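; Player pawn for a bar of soap that is aimed, launched and slides around until it wears away.
; Before launch it moves along world Y while holding Jump oscillates Power; release fires it along the camera's flattened forward.
; Tick sweeps it by Velocity times Power, mirrors off hit normals and drains HP, shrinking capsule or mesh until it stops.
; Overlapping BP_Water gradually rotates Velocity by a random angle, one degree per tick.
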(event `EnhancedInput|/Game/ThirdPerson/Input/Actions/IA_Look`
  (params (ActionValue :type "Vector2D Structure") (ElapsedSeconds :type "Float (double-precision)") (TriggeredSeconds :type "Float (double-precision)") (InputAction :type "InputAction Object Reference" :default "/Game/ThirdPerson/Input/Actions/IA_Look.IA_Look"))
  ;[1 1 1] カメラ操作
  (:`Triggered`
    (`self.AddControllerYawInput` ActionValue_X)
    (`self.AddControllerPitchInput` ActionValue_Y)))

(event `EnhancedInput|/Game/ThirdPerson/Input/Actions/IA_Move`
  (params (ActionValue :type "Vector2D Structure") (ElapsedSeconds :type "Float (double-precision)") (TriggeredSeconds :type "Float (double-precision)") (InputAction :type "InputAction Object Reference" :default "/Game/ThirdPerson/Input/Actions/IA_Move.IA_Move"))
  ;[1 1 1] 移動
  (:`Triggered`
    (if (not (`self.IsStart`))
      (`self.AddMovementInput` (0.0 1.0 0.0) ActionValue_X))))

(event `EnhancedInput|/Game/ThirdPerson/Input/Actions/IA_Jump`
  (params (ActionValue :type Boolean) (ElapsedSeconds :type "Float (double-precision)") (TriggeredSeconds :type "Float (double-precision)") (InputAction :type "InputAction Object Reference" :default "/Game/ThirdPerson/Input/Actions/IA_Jump.IA_Jump"))
  (:`Triggered`
    (if (`self.IsUp`)
      (set `self.Power` (+ (`self.Power`) 0.5))
      (if (> (`self.Power`) 49.0)
        (set `self.IsUp` false))
      (else
        (set `self.Power` (+ (`self.Power`) -0.5))
        (if (< (`self.Power`) 1.0)
          (set `self.IsUp` true)))))
  (:`Completed`
    (set `self.IsStart` true)
    (set `self.Velocity` (`KismetMathLibrary.Vector_Normal2D` (`SceneComponent.GetForwardVector` (`self.Camera`))))))

(event `self.ReceiveBeginPlay`)

(event `self.ReceiveTick`
  (params (DeltaSeconds :type "Float (single-precision)"))
  (bind _returnvalue (/ (`self.HP`) 3.5))
  (bind _returnvalue_2 (/ (`self.HP`) 100.0))
  (if (`self.IsStart`)
    (`|ExecutionSequence`
      (:`then_0`
        (bind _sweephitresult (`self.K2_SetActorLocation` (+ (`self.K2_GetActorLocation`) (* (`self.Velocity`) (`self.Power`))) true))
        (set `self.Velocity` (`KismetMathLibrary.MirrorVectorByNormal` (`self.Velocity`) (`.ImpactNormal` (`GameplayStatics.BreakHitResult` _sweephitresult))))
        (set `self.HP` (- (`self.HP`) 0.1))
        (if (<= (`self.HP`) 35.0)
          (`SceneComponent.SetRelativeScale3D` (`self.SoapMesh`) (`KismetMathLibrary.MakeVector` _returnvalue _returnvalue _returnvalue))
          (else
            (`SceneComponent.SetRelativeScale3D` (`self.CapsuleComponent`) (`KismetMathLibrary.MakeVector` _returnvalue_2 _returnvalue_2 _returnvalue_2))))
        (if (< (`self.HP`) 1.0)
          (set `self.IsStart` false)
          (set `self.IsActive` false)))
      (:`then_1`
        (if (>= (`self.AngleDegree`) (`self.NowAngle`))
          (set `self.NowAngle` (+ (`self.NowAngle`) 1.0))
          (bind _changedvector (`self.ChangeVectorForAngle` (`self.OriginalVelocity`) (`self.NowAngle`)))
          (set `self.Velocity` _changedvector)
          (`KismetSystemLibrary.PrintString` "Hello")))
      (:`then_2`
        (if (`self.IsActive`)
          (`SceneComponent.SetHiddenInGame` (`self.SoapMesh`) true false)
          (else
            (`SceneComponent.SetHiddenInGame` (`self.SoapMesh`) false false)))))))

(event `self.Box.OnComponentBeginOverlap`
  (params (OverlappedComponent :type "PrimitiveComponent Object Reference") (OtherActor :type "Actor Object Reference") (OtherComp :type "PrimitiveComponent Object Reference") (OtherBodyIndex :type Integer) (bFromSweep :type Boolean) (SweepResult :type "HitResult Structure (by ref)"))
  (cast `/Game/IGDA_Game/StageGimmick/Water/BP_Water` OtherActor)
  (`KismetSystemLibrary.PrintString` "Hello")
  (set `self.AngleDegree` (`KismetMathLibrary.RandomFloatInRange` 10.0 30.0))
  (set `self.NowAngle` 0.0)
  (set `self.OriginalVelocity` (`self.Velocity`)))

(fn `ChangeVectorForAngle`
  (params (Vector :type "Vector Structure") (Angle :type "Float (double-precision)"))
  (returns (ChangedVector :type "Vector Structure"))
  (bind _returnvalue (`KismetMathLibrary.DegreesToRadians` Angle))
  (bind _returnvalue_2 (`KismetMathLibrary.Cos` _returnvalue))
  (bind _returnvalue_3 (`KismetMathLibrary.Sin` _returnvalue))
  (return (`KismetMathLibrary.MakeVector` (- (* _returnvalue_2 Vector_X) (* _returnvalue_3 Vector_Y)) (+ (* _returnvalue_3 Vector_X) (* _returnvalue_2 Vector_Y)))))

(fn `UserConstructionScript`)