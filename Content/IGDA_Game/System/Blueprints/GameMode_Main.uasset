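; Main game mode that respawns dead players, enforces the session player cap and handles travel to the matching room.
; On login it kicks the last PlayerArray entry when over GameInstance MaxPlayers, or loads saved GameState and flags everyone logged in when full.
; Logouts after that update MaxPlayers from the current player count.
; OpenNextLevel clears its logged-in flag, saves GameState and issues a servertravel console command to Level_MatchingRoom.
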(event `self.ReceiveBeginPlay`
  (add `self.OnPlayerDied` (delegate `PlayerDied`)))

(event `PlayerDied` :!signature `self.OnPlayerDied`
  (params (Character :type "Character Object Reference"))
  (`self.RestartPlayer` (`Pawn.GetController` Character)))

(event `self.K2_PostLogin`
  (params (NewPlayer :type "PlayerController Object Reference"))
  (bind _returnvalue (`GameplayStatics.GetGameState`))
  ;[1 1 1] ログインがあったとき、プレイヤー数が上限に達していたときの自動キック処理と、セッションメンバー全員がログインしたときのGameState読み出し処理
  (`|ExecutionSequence`
    (:`then_0`
      (bind _asgame_instance_main (cast `/Game/IGDA_Game/System/Blueprints/GameInstance_Main` (`GameplayStatics.GetGameInstance`)))
      (bind _asgame_state_main (cast `/Game/IGDA_Game/System/Blueprints/GameState_Main` _returnvalue))
      (bind _num (`/Game/IGDA_Game/System/Blueprints/GameState_Main.GetCurrentPlayersNum` _asgame_state_main))
      (if (> _num (`/Game/IGDA_Game/System/Blueprints/GameInstance_Main.MaxPlayers` _asgame_instance_main))
        (for _array_element (`GameStateBase.PlayerArray` _returnvalue)
          _)
        (bind _asplayer_controller_main (cast `/Game/IGDA_Game/System/Blueprints/PlayerController_Main` (`PlayerState.GetPlayerController` _array_element)))
        (`/Game/IGDA_Game/System/Blueprints/PlayerController_Main.Kick` _asplayer_controller_main)))
    (:`then_1`
      (bind _asgame_instance_main_2 (cast `/Game/IGDA_Game/System/Blueprints/GameInstance_Main` (`GameplayStatics.GetGameInstance`)))
      (bind _asgame_state_main_2 (cast `/Game/IGDA_Game/System/Blueprints/GameState_Main` (`GameplayStatics.GetGameState`)))
      (bind _num_2 (`/Game/IGDA_Game/System/Blueprints/GameState_Main.GetCurrentPlayersNum` _asgame_state_main_2))
      (if (== _num_2 (`/Game/IGDA_Game/System/Blueprints/GameInstance_Main.MaxPlayers` _asgame_instance_main_2))
        (`/Game/IGDA_Game/System/Blueprints/GameInstance_Main.LoadGameState` _asgame_instance_main_2)
        (set `self.isAllPlayerLoggedIn` true)
        (bind _asgame_state_main_3 (cast `/Game/IGDA_Game/System/Blueprints/GameState_Main` (`GameplayStatics.GetGameState`)))
        (set `/Game/IGDA_Game/System/Blueprints/GameState_Main.IsAllPlayerLoggedIn` true _asgame_state_main_3)))))

(event `self.K2_OnLogout`
  (params (ExitingController :type "Controller Object Reference"))
  ;[1 1 1] ログアウトが起きたとき、プレイヤー数の上限を更新する
  (if (`self.isAllPlayerLoggedIn`)
    (bind _asgame_instance_main (cast `/Game/IGDA_Game/System/Blueprints/GameInstance_Main` (`GameplayStatics.GetGameInstance`)))
    (bind _asgame_state_main (cast `/Game/IGDA_Game/System/Blueprints/GameState_Main` (`GameplayStatics.GetGameState`)))
    (bind _num (`/Game/IGDA_Game/System/Blueprints/GameState_Main.GetCurrentPlayersNum` _asgame_state_main))
    (bind _result (`/Engine/EditorBlueprintResources/StandardMacros.DecrementInt` _num)
      (:`  `
        (set `/Game/IGDA_Game/System/Blueprints/GameInstance_Main.MaxPlayers` _result _asgame_instance_main)))))

(event `OpenNextLevel`
  ;[1 1 1] カスタムイベント - GameStateを保存して次のレベルへ遷移する
  (set `self.isAllPlayerLoggedIn` false)
  (bind _asgame_instance_main (cast `/Game/IGDA_Game/System/Blueprints/GameInstance_Main` (`GameplayStatics.GetGameInstance`)))
  (`/Game/IGDA_Game/System/Blueprints/GameInstance_Main.SaveGameState` _asgame_instance_main)
  (for _array_element (`GameStateBase.PlayerArray` (`GameplayStatics.GetGameState`))
    (if (`self.HasAuthority` _array_element)
      (`/Engine/EditorBlueprintResources/StandardMacros.DoOnce` false
        (:`Completed`
          (`KismetSystemLibrary.ExecuteConsoleCommand` (`KismetStringLibrary.Concat_StrStr` "servertravel " "/Game/shimabukuro/Menu/Maps/Level_MatchingRoom") (`PlayerState.GetPlayerController` _array_element)))))))

(fn `UserConstructionScript`)